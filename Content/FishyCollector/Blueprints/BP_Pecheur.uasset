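; BP_Pecheur is the fisherman player Blueprint, which handles startup setup for the fish-collecting game.
; On BeginPlay it initializes a shared registry, fetched through the game instance, with the DA_PokedexRegistre Pokédex data.
; Outside the Menu level, it also creates and displays the player HUD and adds the classic fishing rod to the owned rods.
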(event `self.ReceiveBeginPlay`
  (`PokedexManager.InitialiserRegistre` (`PokedexManager.GetInstance` (`GameplayStatics.GetGameInstance`)) "/Game/FishyCollector/Poisson/DA/DA_PokedexRegistre.DA_PokedexRegistre")
  (bind _returnvalue (`GameplayStatics.GetCurrentLevelName` true))
  (if (not (`KismetStringLibrary.EqualEqual_StrStr` _returnvalue "Menu"))
    (bind _returnvalue_2 (`|CreateWidget` "/Game/FishyCollector/UI/HUD/WBP_HUD_CS.WBP_HUD_CS_C"))
    (bind _output_get (set `self.HUD_Joueur` _returnvalue_2))
    (`UserWidget.AddToViewport` _output_get 0)
    (`KismetArrayLibrary.Array_Add` (`self.OwnedFishingRods`) "/Game/FishyCollector/Data/ClassicFishingRod.ClassicFishingRod")))

(fn `UserConstructionScript`)
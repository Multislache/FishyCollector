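; BP_ZoneDePeche is a fishing zone that turns fishing availability on and off for the player's BP_Pecheur character.
; When its ZoneDePeche component begins an overlap, it sets the character's fishing-zone flag and adds a new WBP_ZoneDePeche widget to the viewport.
; When the overlap ends, it clears the flag and removes the widget.
; Both handlers act on player character 0 without checking which actor overlapped.
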(event `self.ZoneDePeche.OnComponentBeginOverlap`
  (params (OverlappedComponent :type "PrimitiveComponent Object Reference") (OtherActor :type "Actor Object Reference") (OtherComp :type "PrimitiveComponent Object Reference") (OtherBodyIndex :type Integer) (bFromSweep :type Boolean) (SweepResult :type "HitResult Structure (by ref)"))
  (bind _asbp_pecheur (cast `/Game/FishyCollector/Blueprints/BP_Pecheur` (`GameplayStatics.GetPlayerCharacter` 0)))
  (`FishyCollectorCharacter.SetFishingZoneActive` _asbp_pecheur true)
  (bind _returnvalue (`|CreateWidget` "/Game/FishyCollector/UI/WBP_ZoneDePeche.WBP_ZoneDePeche_C"))
  (bind _output_get (set `self.WidgetZDP` _returnvalue))
  (`UserWidget.AddToViewport` _output_get 0))

(event `self.ZoneDePeche.OnComponentEndOverlap`
  (params (OverlappedComponent :type "PrimitiveComponent Object Reference") (OtherActor :type "Actor Object Reference") (OtherComp :type "PrimitiveComponent Object Reference") (OtherBodyIndex :type Integer))
  (bind _widgetzdp (`self.WidgetZDP`))
  (bind _asbp_pecheur (cast `/Game/FishyCollector/Blueprints/BP_Pecheur` (`GameplayStatics.GetPlayerCharacter` 0)))
  (`FishyCollectorCharacter.SetFishingZoneActive` _asbp_pecheur false)
  (`/Engine/EditorBlueprintResources/StandardMacros.IsValid` _widgetzdp
    (:`Is Valid`
      (`Widget.RemoveFromParent` _widgetzdp))))

(fn `UserConstructionScript`)
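; BP_Pecheur1 is the fisherman Blueprint of FishyCollector, set up according to the current level.
; On BeginPlay it initializes the game instance's registry from the Pokedex registry data asset.
; In the Menu level it plays the fishing idle montage at a near-frozen rate as a posed figure.
; In other levels it creates and shows the player HUD and adds the classic rod to the owned fishing rods.
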(event `self.ReceiveBeginPlay`
  (`PokedexManager.InitialiserRegistre` (`PokedexManager.GetInstance` (`GameplayStatics.GetGameInstance`)) "/Game/FishyCollector/Poisson/DA/DA_PokedexRegistre.DA_PokedexRegistre")
  (bind _returnvalue (`GameplayStatics.GetCurrentLevelName` true))
  (if (`KismetStringLibrary.EqualEqual_StrStr` _returnvalue "Menu")
    (`|PlayMontage` (`self.Mesh`) "/Game/ST_Characters_JC/Animation/Female/Fishing_Idle_Montage.Fishing_Idle_Montage" 0.001)
    (else
      (bind _returnvalue_2 (`|CreateWidget` "/Game/FishyCollector/UI/HUD/WBP_HUD_CS.WBP_HUD_CS_C"))
      (bind _output_get (set `self.HUD_Joueur` _returnvalue_2))
      (`UserWidget.AddToViewport` _output_get 0)
      (`KismetArrayLibrary.Array_Add` (`self.OwnedFishingRods`) "/Game/FishyCollector/Data/ClassicFishingRod.ClassicFishingRod"))))

(fn `UserConstructionScript`)
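; BP_FishingRodStorage is a fishing rod storage actor that BP_Pecheur can interact with when nearby.
; Entering its collision box registers it as the fisher's nearby storage and shows a newly created WBP_InteractStockage prompt.
; Any end overlap clears that reference on player character 0, without checking which actor left, and removes the prompt.
; The file only handles proximity, with no storage logic of its own.
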(event `self.BoxCollision.OnComponentBeginOverlap`
  (params (OverlappedComponent :type "PrimitiveComponent Object Reference") (OtherActor :type "Actor Object Reference") (OtherComp :type "PrimitiveComponent Object Reference") (OtherBodyIndex :type Integer) (bFromSweep :type Boolean) (SweepResult :type "HitResult Structure (by ref)"))
  (bind _asbp_pecheur (cast `/Game/FishyCollector/Blueprints/BP_Pecheur` OtherActor))
  (set `FishyCollectorCharacter.NearbyStorage` self _asbp_pecheur)
  (`FishyCollectorCharacter.SetNearbyStorage` _asbp_pecheur self)
  (bind _returnvalue (`|CreateWidget` "/Game/FishyCollector/UI/StockageCAP/WBP_InteractStockage.WBP_InteractStockage_C"))
  (bind _output_get (set `self.WBPInteractStockage` _returnvalue))
  (`UserWidget.AddToViewport` _output_get 0)
  (set `self.InteractWidgetInstance` _output_get))

(event `self.BoxCollision.OnComponentEndOverlap`
  (params (OverlappedComponent :type "PrimitiveComponent Object Reference") (OtherActor :type "Actor Object Reference") (OtherComp :type "PrimitiveComponent Object Reference") (OtherBodyIndex :type Integer))
  (bind _asbp_pecheur (cast `/Game/FishyCollector/Blueprints/BP_Pecheur` (`GameplayStatics.GetPlayerCharacter` 0)))
  (`FishyCollectorCharacter.SetNearbyStorage` _asbp_pecheur null)
  (set `FishyCollectorCharacter.NearbyStorage` null _asbp_pecheur)
  (`Widget.RemoveFromParent` (`self.WBPInteractStockage`)))

(fn `UserConstructionScript`)